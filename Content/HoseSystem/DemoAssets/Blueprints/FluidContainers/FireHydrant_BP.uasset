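; Fire hydrant demo asset for the hose system, acting as a fluid container with a single pumpable HoseConnection.
; Container functions forward pump queries and start/stop calls to that connection, refusing to start when it is connected as an output.
; Pump state changes drive the particle system, which plays only while pumping and the attached hose's HoseConnected flag is false.
; GetAllConnections is a stub that returns nothing.
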(event `self.HoseConnection.PumpStateChanged`
  (params (IsPumping :type Boolean))
  (if IsPumping
    (`ActorComponent.SetActive` (`self.ParticleSystem`) (not (`/Game/HoseSystem/Blueprints/Container_Connection.GetConnectedHose` (`self.HoseConnection`))) false)
    (else
      (`ActorComponent.SetActive` (`self.ParticleSystem`) false false))))

(fn `GetAllConnections`
  (returns (Connections :type "Array of /Game/HoseSystem/Blueprints/Container_Connection Object Reference"))
  (return))

(fn `GetContainerConnection`
  (params (Location :type "Transform Structure"))
  (returns (Connection :type "/Game/HoseSystem/Blueprints/Container_Connection Object Reference"))
  (return (`self.HoseConnection`)))

(fn `GetIsAnyPumping`
  (returns (IsPumping :type Boolean))
  (return (`/Game/HoseSystem/Blueprints/Container_Connection.GetIsPumping` (`self.HoseConnection`))))

(fn `StartAllPumps`
  (returns (Success :type Boolean))
  (bind _hoseconnection (`self.HoseConnection`))
  (if (not (`/Game/HoseSystem/Blueprints/Container_Connection.GetIsConnectedAsOutput` _hoseconnection))
    (`/Game/HoseSystem/Blueprints/Container_Connection.StartPump` _hoseconnection)
    (return true)
    (else
      (return false))))

(fn `StopAllPumps`
  (returns (Success :type Boolean))
  (`/Game/HoseSystem/Blueprints/Container_Connection.StopPump` (`self.HoseConnection`))
  (return true))

(fn `UserConstructionScript`)