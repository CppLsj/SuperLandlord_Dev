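; Water tank actor for the hose system that stores fluid and exposes a single hose connection with pump controls.
; The authority seeds the starting fill, and content changes drive a fill mesh that eases toward the new level.
; A full tank stops all pumps through the connection.
; Pump state swaps red and green indicator lights and sprays water when the pumping hose's HoseConnected flag is false.
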(event `self.ReceiveTick`
  (params (DeltaSeconds :type "Float (single-precision)"))
  (bind (_returnvalue_x _returnvalue_y _returnvalue_z) (`KismetMathLibrary.BreakVector` (`SceneComponent.K2_GetComponentScale` (`self.WaterTank_WaterFill_Mesh`))))
  (`SceneComponent.SetWorldScale3D` (`self.WaterTank_WaterFill_Mesh`) (`KismetMathLibrary.MakeVector` 1.0 1.0 (`KismetMathLibrary.Lerp` _returnvalue_z (`self.FluidPercent`) DeltaSeconds))))

(event `self.ReceiveBeginPlay`
  (`self.UpdateLights` false)
  (`/Engine/EditorBlueprintResources/ActorMacros.Switch Has Authority`
    (:`Authority`
      (`/Game/HoseSystem/Blueprints/Container_Component.AddContents` (`self.WaterTank`) (`self.SpawnTankFill`)))))

(event `self.WaterTank.ContentsChange`
  (params (NewFluid :type "Float (single-precision)"))
  (set `self.FluidPercent` (/ NewFluid (`/Game/HoseSystem/Blueprints/Container_Component.MaxCapacity` (`self.WaterTank`)))))

(event `self.WaterTank.ContentsFull`
  (message `/Game/HoseSystem/Blueprints/Connections_Interface.StopAllPumps` (`self.HoseConnection`)))

(event `self.HoseConnection.PumpStateChanged`
  (params (IsPumping :type Boolean))
  (`self.UpdateLights` IsPumping)
  (if IsPumping
    (`ActorComponent.SetActive` (`self.HoseSpray`) (not (`/Game/HoseSystem/Blueprints/Container_Connection.GetConnectedHose` (`self.HoseConnection`))) false)
    (else
      (`ActorComponent.SetActive` (`self.HoseSpray`) false false))))

(event `UpdateLights`
  (params (Pump :type Boolean))
  (`PrimitiveComponent.SetMaterial` (`self.OnLight`) 0 (select `bool` Pump :`false` "/Game/HoseSystem/DemoAssets/Materials/Generic/Lights/Light_Green.Light_Green" :`true` "/Game/HoseSystem/DemoAssets/Materials/Generic/Lights/Light_Green_Lit.Light_Green_Lit" :!type "MaterialInterface Object Reference"))
  (`PrimitiveComponent.SetMaterial` (`self.OffLight`) 0 (select `bool` Pump :`false` "/Game/HoseSystem/DemoAssets/Materials/Generic/Lights/Light_Red_Lit.Light_Red_Lit" :`true` "/Game/HoseSystem/DemoAssets/Materials/Generic/Lights/Light_Red.Light_Red" :!type "MaterialInterface Object Reference")))

(fn `GetAllConnections`
  (returns (Connections :type "Array of /Game/HoseSystem/Blueprints/Container_Connection Object Reference"))
  (return))

(fn `GetContainerConnection`
  (params (Location :type "Transform Structure"))
  (returns (Connection :type "/Game/HoseSystem/Blueprints/Container_Connection Object Reference"))
  (return (`self.HoseConnection`)))

(fn `GetIsAnyPumping`
  (returns (IsPumping :type Boolean))
  (return (`/Game/HoseSystem/Blueprints/Container_Connection.GetIsPumping` (`self.HoseConnection`))))

(fn `StartAllPumps`
  (returns (Success :type Boolean))
  (bind _hoseconnection (`self.HoseConnection`))
  (if (not (`/Game/HoseSystem/Blueprints/Container_Connection.GetIsConnectedAsOutput` _hoseconnection))
    (`/Game/HoseSystem/Blueprints/Container_Connection.StartPump` _hoseconnection)
    (return true)
    (else
      (return false))))

(fn `StopAllPumps`
  (returns (Success :type Boolean))
  (`/Game/HoseSystem/Blueprints/Container_Connection.StopPump` (`self.HoseConnection`))
  (return true))

(fn `UserConstructionScript`
  (`SceneComponent.SetWorldScale3D` (`self.WaterTank_WaterFill_Mesh`) (`KismetMathLibrary.MakeVector` 1.0 1.0 (/ (`self.SpawnTankFill`) (`/Game/HoseSystem/Blueprints/Container_Component.MaxCapacity` (`self.WaterTank`))))))