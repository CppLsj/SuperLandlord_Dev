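; Mounted fluid tank for the hose system demo, with one hose connection and weight that follows its contents.
; Content changes update body mass and soften the constraint's linear drive to fake load, since position drives ignore mass.
; Tick eases the fill mesh toward the current level, starting from the spawn fill.
; Pumping stops when full and sprays if the hose is unconnected; most container query and pump functions are stubs.
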(event `self.ReceiveBeginPlay`
  ;[1 1 1] Physics weight change with contents amount
  (`self.UpdateContainerWeight` :!label _label))

(event `self.Container_Component.ContentsChange`
  (params (NewFluid :type "Float (single-precision)"))
  ;[1 1 1] Physics weight change with contents amount
  (goto _label))

(event `self.Container_Component.ContentsFull`
  (`/Game/HoseSystem/Blueprints/Container_Connection.StopPump` (`self.HoseConnection`)))

(event `self.HoseConnection.PumpStateChanged`
  (params (IsPumping :type Boolean))
  (if IsPumping
    (`ActorComponent.SetActive` (`self.HoseSpray`) (not (`/Game/HoseSystem/Blueprints/Container_Connection.GetConnectedHose` (`self.HoseConnection`))) false)
    (else
      (`ActorComponent.SetActive` (`self.HoseSpray`) false false))))

(event `self.ReceiveTick`
  (params (DeltaSeconds :type "Float (single-precision)"))
  (`self.UpdateTankVisual`))

(fn `GetAllConnections`
  (returns (Connections :type "Array of /Game/HoseSystem/Blueprints/Container_Connection Object Reference"))
  (return))

(fn `GetContainerConnection`
  (params (Location :type "Transform Structure"))
  (returns (Connection :type "/Game/HoseSystem/Blueprints/Container_Connection Object Reference"))
  (return (`self.HoseConnection`)))

(fn `GetIsAnyPumping`
  (returns (IsPumping :type Boolean))
  (return false))

(fn `StartAllPumps`
  (returns (Success :type Boolean))
  (return false))

(fn `StopAllPumps`
  (returns (Success :type Boolean))
  (return false))

(fn `UpdateContainerWeight`
  (locals (NewMass :type "Float (double-precision)" :default 0.0))
  (bind _watertank_carmounted (`self.WaterTank_CarMounted`))
  (bind _output_get (set `local.NewMass` (`KismetMathLibrary.MapRangeClamped` (`/Game/HoseSystem/Blueprints/Container_Component.CurrentContents` (`self.Container_Component`)) 0.0 100.0 400.0 1400.0)))
  (`PrimitiveComponent.SetMassOverrideInKg` _watertank_carmounted "None" _output_get true)
  (`PrimitiveComponent.WakeRigidBody` _watertank_carmounted "None")
  (bind _constraintactor (`self.ConstraintActor`)
    (:`then`
      ;[1 1 1] I wanted to use soft constraints for this, but they don't work in UE5
      (`PhysicsConstraintComponent.SetLinearDriveParams` (`PhysicsConstraintActor.ConstraintComp` _constraintactor) (`KismetMathLibrary.MapRangeClamped` (`/Game/HoseSystem/Blueprints/Container_Component.CurrentContents` (`self.Container_Component`)) 0.0 100.0 5.0 2.5) 0.0 0.0) ; Position drive ignores mass, so we fake it
    )
    (:`else`)))

(fn `UpdateTankVisual`
  (bind (_returnvalue_x _returnvalue_y _returnvalue_z) (`KismetMathLibrary.BreakVector` (`SceneComponent.K2_GetComponentScale` (`self.WaterTank_WaterFill`))))
  (`SceneComponent.SetWorldScale3D` (`self.WaterTank_WaterFill`) (`KismetMathLibrary.MakeVector` 0.21 0.21 (`KismetMathLibrary.Lerp` _returnvalue_z (* (/ (`/Game/HoseSystem/Blueprints/Container_Component.CurrentContents` (`self.Container_Component`)) (`/Game/HoseSystem/Blueprints/Container_Component.MaxCapacity` (`self.Container_Component`))) 0.21) (`GameplayStatics.GetWorldDeltaSeconds`)))))

(fn `UserConstructionScript`
  (`SceneComponent.SetWorldScale3D` (`self.WaterTank_WaterFill`) (`KismetMathLibrary.MakeVector` 0.21 0.21 (* (/ (`self.SpawnTankFill`) (`/Game/HoseSystem/Blueprints/Container_Component.MaxCapacity` (`self.Container_Component`))) 0.21)))
  (set `/Game/HoseSystem/Blueprints/Container_Component.CurrentContents` (`self.SpawnTankFill`) (`self.Container_Component`)))