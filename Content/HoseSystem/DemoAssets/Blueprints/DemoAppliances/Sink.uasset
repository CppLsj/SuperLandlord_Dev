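; Demo sink appliance for the hose system that sprays while its hose connection is pumping.
; Player interaction toggles the pump when the sink is connected as output, or prints a warning if the hose is backwards.
; Tick watches the pumping state and switches the spray and fading audio on changes.
; Of the container and pump functions, only StartAllPumps acts; the others are stubs, including StopAllPumps.
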(event `/Game/HoseSystem/Blueprints/Connections_Interface.PlayerInteract`
  (params (SpecificConnection :type "/Game/HoseSystem/Blueprints/Container_Connection Object Reference"))
  (bind _hoseconnection (`self.HoseConnection`))
  (if (`/Game/HoseSystem/Blueprints/Container_Connection.GetIsConnectedAsOutput` _hoseconnection)
    (`/Game/HoseSystem/Blueprints/Container_Connection.TogglePump` _hoseconnection)
    (elif (`/Game/HoseSystem/Blueprints/Container_Connection.GetConnectedHose` _hoseconnection)
      (`KismetSystemLibrary.PrintString` "Hose is connected backwards!" true false))))

(event `self.ReceiveTick`
  (params (DeltaSeconds :type "Float (single-precision)"))
  (bind _audio (`self.Audio`))
  (bind _ispumping (`/Game/HoseSystem/Blueprints/Container_Connection.GetIsPumping` (`self.HoseConnection`)))
  (if (!= _ispumping (`self.IsActive`))
    (bind _output_get (set `self.IsActive` _ispumping))
    (`ActorComponent.SetActive` (`self.Spray`) _output_get false)
    (if (`self.IsActive`)
      (`AudioComponent.FadeIn` _audio 0.5 1.0 0.0 "Linear")
      (else
        (`AudioComponent.FadeOut` _audio 0.5 0.0 "Linear")))))

(fn `GetAllConnections`
  (returns (Connections :type "Array of /Game/HoseSystem/Blueprints/Container_Connection Object Reference"))
  (return))

(fn `GetContainerConnection`
  (params (Location :type "Transform Structure"))
  (returns (Connection :type "/Game/HoseSystem/Blueprints/Container_Connection Object Reference"))
  (return null))

(fn `GetIsAnyPumping`
  (returns (IsPumping :type Boolean))
  (return false))

(fn `StartAllPumps`
  (returns (Success :type Boolean))
  (`/Game/HoseSystem/Blueprints/Container_Connection.StartPump` (`self.HoseConnection`))
  (return true))

(fn `StopAllPumps`
  (returns (Success :type Boolean))
  (return false))

(fn `UserConstructionScript`)