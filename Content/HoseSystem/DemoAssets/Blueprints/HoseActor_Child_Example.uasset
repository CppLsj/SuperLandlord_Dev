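; Example child of the hose actor that automatically hooks a hose up between an Input and an Output object at BeginPlay.
; After the parent's setup, it connects to the Input's container connection and, only if that exists, to the Output's.
; With both ends connected and no predefined spline path, it creates a centered anchor point, useful when the connections start close together.
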(event `self.ReceiveBeginPlay`
  (bind _input (`self.Input`))
  (bind _output (`self.Output`))
  (`parent.ReceiveBeginPlay`)
  (`/Engine/EditorBlueprintResources/StandardMacros.IsValid` _input
    (:`Is Valid`
      (`self.SetInputConnection` (`/Game/HoseSystem/DemoAssets/Blueprints/PhysicsCube.Container_Connection` _input))
      (`/Engine/EditorBlueprintResources/StandardMacros.IsValid` _output
        (:`Is Valid`
          (`self.SetOutputConnection` (`/Game/HoseSystem/DemoAssets/Blueprints/PhysicsCube.Container_Connection` _output))
          (`/Engine/EditorBlueprintResources/StandardMacros.IsValid` (`self.PredefinedSplinePath`)
            (:`Is Not Valid`
              (`self.CreateCenteredAnchorPoint`) ; This can be useful when creating hoses where the \nconnections start close together
            )))))))

(fn `ActiveConnectionDestroyed`
  (`parent.ActiveConnectionDestroyed`))

(fn `UserConstructionScript`
  (`parent.UserConstructionScript`))