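; Hose nozzle actor for the hose system demo, which shows spray particles and fades audio while its hose input is pumping.
; When simulating physics and pumping, it applies backward thrust each tick and runs a looping timer of random angular kicks to whip the nozzle around.
; ConnectedHose's OnRep links the hose output to the nozzle input, and a disconnect destroys the actor.
; SetPhysics toggles simulation and collision mode.
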(event `SetPhysics`
  (params (NewPhysics :type Boolean))
  (bind _staticmesh (`self.StaticMesh`))
  (bind _staticmesh_2 (`self.StaticMesh`))
  (if NewPhysics
    (`PrimitiveComponent.SetCollisionEnabled` _staticmesh_2 "QueryAndPhysics")
    (`PrimitiveComponent.SetSimulatePhysics` _staticmesh_2 true)
    (else
      (`PrimitiveComponent.SetSimulatePhysics` _staticmesh false)
      (`PrimitiveComponent.SetCollisionEnabled` _staticmesh "PhysicsOnly"))))

(event `self.NozzleHoseInput.HoseDisconnected`
  (`self.K2_DestroyActor`))

(event `PunchHose`
  (`PrimitiveComponent.AddAngularImpulseInDegrees` (`self.StaticMesh`) (* (`KismetMathLibrary.RandomUnitVector`) 750.0) "None" true))

(event `self.ReceiveTick`
  (params (DeltaSeconds :type "Float (single-precision)"))
  (bind _audio (`self.Audio`))
  (bind _ispumping (`/Game/HoseSystem/Blueprints/Container_Connection.GetIsPumping` (`self.NozzleHoseInput`)))
  (if (!= _ispumping (`self.IsPumping`))
    (bind _output_get (set `self.IsPumping` _ispumping))
    (`ActorComponent.SetActive` (`self.ParticleSystem`) _output_get false)
    (if (`self.IsPumping`)
      (`AudioComponent.FadeIn` _audio 0.25 1.0 0.0 "Linear")
      (else
        (`AudioComponent.FadeOut` _audio 0.25 0.0 "Linear"))))
  (if (and (`SceneComponent.IsSimulatingPhysics` (`self.StaticMesh`) "None") (`self.IsPumping`))
    (`PrimitiveComponent.AddImpulse` (`self.StaticMesh`) (* (* (`SceneComponent.GetForwardVector` (`self.StaticMesh`)) -7700) DeltaSeconds) "None" false)
    (if (not (`KismetSystemLibrary.K2_IsTimerActiveHandle` (`self.HosePunchTimer`)))
      (bind _returnvalue (`KismetSystemLibrary.K2_SetTimerDelegate` (delegate `PunchHose`) 0.1 true))
      (set `self.HosePunchTimer` _returnvalue))
    (else
      (`KismetSystemLibrary.K2_ClearAndInvalidateTimerHandle` (`self.HosePunchTimer`)))))

(fn `GetConnectedHose`
  (returns (ConnectedHose :type "/Game/HoseSystem/Blueprints/HoseActor Object Reference"))
  (return (`self.ConnectedHose`)))

(fn `OnRep_ConnectedHose`
  (bind _connectedhose (`self.ConnectedHose`))
  (`/Engine/EditorBlueprintResources/StandardMacros.IsValid` _connectedhose
    (:`Is Valid`
      (`/Game/HoseSystem/Blueprints/HoseActor.SetOutputConnection` _connectedhose (`self.NozzleHoseInput`)))))

(fn `SetConnectedHose`
  (params (ConnectedHose :type "/Game/HoseSystem/Blueprints/HoseActor Object Reference"))
  (bind _output_get (set `self.ConnectedHose` ConnectedHose))
  (`/Engine/EditorBlueprintResources/StandardMacros.IsValid` _output_get))

(fn `UserConstructionScript`)