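; Actor component in the hose system that stores an amount of fluid up to a capacity, with optional infinite supply.
; Adding past capacity either fills and spills the excess or, without overflow, rejects the whole amount, signaling full in both cases.
; Removal returns what is available, signaling empty when a request exceeds it.
; A RepNotify on contents broadcasts changes, and a helper totals per-second output of pumping connections.
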(fn `AddContents`
  (params (AddAmount :type "Float (double-precision)"))
  (locals (TotalNewContents :type "Float (double-precision)" :default 0.0))
  (bind _maxcapacity (`self.MaxCapacity`))
  (bind _output_get (set `local.TotalNewContents` (+ AddAmount (`self.CurrentContents`))))
  (if (> _output_get (`self.MaxCapacity`))
    (if (`self.CanOverflow`)
      (set `self.CurrentContents` _maxcapacity)
      (`self.ContentsSpill` (- (`local.TotalNewContents`) _maxcapacity))
      (`self.ContentsFull`)
      (else
        (`self.ContentsFull`)))
    (else
      (set `self.CurrentContents` (`KismetMathLibrary.FClamp` _output_get 0.0 (`self.MaxCapacity`))))))

(fn `GetIsEmpty`
  (returns (IsEmpty :type Boolean))
  (return (and (not (`self.InfiniteContents`)) (<= (`self.CurrentContents`) 0.0))))

(fn `GetTotalOutput`
  (params (Connections :type "Array of /Game/HoseSystem/Blueprints/Container_Connection Object Reference"))
  (returns (ContentsPerSec :type "Float (double-precision)"))
  (locals (TotalPerSec :type "Float (double-precision)"))
  (for _array_element Connections
    (if (`/Game/HoseSystem/Blueprints/Container_Connection.GetIsPumping` _array_element)
      (set `local.TotalPerSec` (+ (`local.TotalPerSec`) (`/Game/HoseSystem/Blueprints/Container_Connection.PumpContentsPerSec` _array_element)))))
  (return (`local.TotalPerSec`)))

(fn `OnRep_CurrentContents`
  (`self.ContentsChange` (`self.CurrentContents`)))

(fn `RemoveContents`
  (params (RequestAmount :type "Float (double-precision)"))
  (returns (Took :type Boolean) (TakeAmount :type "Float (double-precision)"))
  (locals (FluidTake :type "Float (double-precision)"))
  (bind _currentcontents (`self.CurrentContents`))
  (if (not (`self.InfiniteContents`))
    (if (<= (`self.CurrentContents`) 0.0)
      (return false 0.0) ; No fluid to take
      (elif (> RequestAmount _currentcontents)
        (bind _output_get (set `local.FluidTake` (`self.CurrentContents`)))
        (set `self.CurrentContents` 0.0)
        (`self.ContentsEmpty`)
        (return true _output_get) ; Not enough fluid for request amount
        (else
          (set `self.CurrentContents` (- _currentcontents RequestAmount))
          (return true RequestAmount) ; Can accommodate full request amount
        )))
    (else
      (return true RequestAmount))))