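; Connection component that links a fluid container to a hose and pumps contents through it.
; Server-authoritative start/stop calls route to the hose's input connection, and the IsPumping RepNotify runs a looping quarter-second timer.
; Each tick moves fluid from the owning container to the output connection's container, respecting non-overflow capacity or reporting a spill without a receiver.
; It can auto-find its owner's container, raises hose and pump state events, and notifies the hose when its owner is destroyed.
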(event `self.ReceiveBeginPlay`
  (`self.AutoFindContainer`)
  (add `Actor.OnDestroyed` (`self.GetOwner`) (delegate `ImBeingDestroyed`)))

(event `ImBeingDestroyed`
  (params (DestroyedActor :type "Actor Object Reference"))
  (bind (_hoseconnected _hose) (`self.GetConnectedHose`))
  (`/Engine/EditorBlueprintResources/StandardMacros.IsValid` _hose
    (:`Is Valid`
      (`/Game/HoseSystem/Blueprints/HoseActor.ActiveConnectionDestroyed` _hose))))

(fn `AutoFindContainer`
  (if (`self.AutoContainer`)
    (`self.SetOwningContainer` (`Actor.GetComponentByClass` (`self.GetOwner`) "/Game/HoseSystem/Blueprints/Container_Component.Container_Component_C"))))

(fn `GetConnectedHose`
  (returns (HoseConnected :type Boolean) (Hose :type "/Game/HoseSystem/Blueprints/HoseActor Object Reference"))
  (bind _hose (`self.Hose`))
  (return (`KismetSystemLibrary.IsValid` _hose) _hose))

(fn `GetIsConnectedAsInput`
  (returns (IsInput :type Boolean))
  (bind _hose (`self.Hose`))
  (`/Engine/EditorBlueprintResources/StandardMacros.IsValid` _hose
    (:`Is Valid`
      (return (== (`/Game/HoseSystem/Blueprints/HoseActor.GetInputConnection` _hose) self)))
    (:`Is Not Valid`
      (return false))))

(fn `GetIsConnectedAsOutput`
  (returns (IsOutput :type Boolean))
  (bind _hose (`self.Hose`))
  (`/Engine/EditorBlueprintResources/StandardMacros.IsValid` _hose
    (:`Is Valid`
      (return (== (`/Game/HoseSystem/Blueprints/HoseActor.GetOutputConnection` _hose) self)))
    (:`Is Not Valid`
      (return false))))

(fn `GetIsPumping`
  (returns (IsPumping :type Boolean))
  (return (or (`self.IsPumping`) (`self.GetIsReceivingPump`))))

(fn `GetIsReceivingPump`
  (returns (IsPumping :type Boolean))
  (bind _hose (`self.Hose`))
  (bind _inputconnection (`/Game/HoseSystem/Blueprints/HoseActor.GetInputConnection` _hose))
  (`/Engine/EditorBlueprintResources/StandardMacros.IsValid` _hose
    (:`Is Valid`
      (`/Engine/EditorBlueprintResources/StandardMacros.IsValid` _inputconnection
        (:`Is Valid`
          (if (`self.GetIsConnectedAsOutput`)
            (return (`self.GetIsPumping` _inputconnection))
            (else
              (return false))))
        (:`Is Not Valid`
          (return false))))
    (:`Is Not Valid`
      (return false))))

(fn `GetMaxContentsToSend`
  (returns (MaxContentsToSend :type "Float (double-precision)"))
  (bind _outputcontainer (`self.GetOutputContainer`))
  (`/Engine/EditorBlueprintResources/StandardMacros.IsValid` _outputcontainer
    (:`Is Valid`
      (if (not (`/Game/HoseSystem/Blueprints/Container_Component.CanOverflow` _outputcontainer))
        (return (- (`/Game/HoseSystem/Blueprints/Container_Component.MaxCapacity` _outputcontainer) (`/Game/HoseSystem/Blueprints/Container_Component.CurrentContents` _outputcontainer)))
        (else
          _)))
    (:`Is Not Valid`
      _))
  (return (`self.PumpContentsPerSec`)))

(fn `GetOutputContainer`
  (returns (OutputContainer :type "/Game/HoseSystem/Blueprints/Container_Component Object Reference"))
  (bind (_hoseconnected _hose) (`self.GetConnectedHose`))
  (bind _outputconnection (`/Game/HoseSystem/Blueprints/HoseActor.GetOutputConnection` _hose))
  (bind _owningcontainer (`self.GetOwningContainer` _outputconnection))
  (if _hoseconnected
    (`/Engine/EditorBlueprintResources/StandardMacros.IsValid` _outputconnection
      (:`Is Valid`
        (`/Engine/EditorBlueprintResources/StandardMacros.IsValid` _owningcontainer
          (:`Is Valid`
            (return _owningcontainer))
          (:`Is Not Valid`
            (return null))))
      (:`Is Not Valid`
        (return null)))
    (else
      (return null))))

(fn `GetOwningContainer`
  (returns (OwningContainer :type "/Game/HoseSystem/Blueprints/Container_Component Object Reference"))
  (return (`self.OwningContainer`)))

(fn `OnRep_Hose`
  (`/Engine/EditorBlueprintResources/StandardMacros.IsValid` (`self.Hose`)
    (:`Is Valid`
      (`self.HoseConnected`))
    (:`Is Not Valid`
      (`self.HoseDisconnected`)))
  (`self.PumpStateChanged` (`self.GetIsPumping`)))

(fn `OnRep_IsPumping`
  (if (`self.IsPumping`)
    (bind _returnvalue (`KismetSystemLibrary.K2_SetTimer` null "Pump" 0.25 true))
    (set `self.PumpTimer` _returnvalue)
    (else
      (`KismetSystemLibrary.K2_ClearAndInvalidateTimerHandle` (`self.PumpTimer`))))
  (`self.PumpStateChanged` (`self.IsPumping`)))

(fn `Pump`
  (bind _owningcontainer (`self.OwningContainer`))
  (bind _returnvalue (`KismetMathLibrary.FClamp` (/ (`self.PumpContentsPerSec`) 4.0) 0.0 (`self.GetMaxContentsToSend`)))
  (`/Engine/EditorBlueprintResources/StandardMacros.IsValid` _owningcontainer
    (:`Is Valid`
      (if (not (`/Game/HoseSystem/Blueprints/Container_Component.GetIsEmpty` _owningcontainer))
        (if (> _returnvalue 0.0)
          (`self.SendContents` _returnvalue))
        (else
          (`self.StopPump` :!label _label))))
    (:`Is Not Valid`
      (goto _label))))

(fn `ReceiveContents`
  (params (Fluid :type "Float (double-precision)"))
  (bind _owningcontainer (`self.OwningContainer`))
  (`/Engine/EditorBlueprintResources/StandardMacros.IsValid` _owningcontainer
    (:`Is Valid`
      (`/Game/HoseSystem/Blueprints/Container_Component.AddContents` _owningcontainer Fluid))
    (:`Is Not Valid`
      (`self.FluidSpilled` Fluid))))

(fn `SendContents`
  (params (Fluid :type "Float (double-precision)"))
  (bind (_hoseconnected _hose) (`self.GetConnectedHose`))
  (bind _owningcontainer (`self.OwningContainer`))
  (bind _outputconnection (`/Game/HoseSystem/Blueprints/HoseActor.GetOutputConnection` _hose))
  (`/Engine/EditorBlueprintResources/StandardMacros.IsValid` _owningcontainer
    (:`Is Valid`
      (bind (_took _takeamount) (`/Game/HoseSystem/Blueprints/Container_Component.RemoveContents` _owningcontainer Fluid))
      (if _took
        (if _hoseconnected
          (`/Engine/EditorBlueprintResources/StandardMacros.IsValid` _outputconnection
            (:`Is Valid`
              (`self.ReceiveContents` _outputconnection _takeamount))
            (:`Is Not Valid`
              (`self.FluidSpilled` _takeamount :!label _label)))
          (else
            (goto _label)))))))

(fn `SetConnectedHose`
  (params (ConnectedHose :type "/Game/HoseSystem/Blueprints/HoseActor Object Reference"))
  (if (`Actor.HasAuthority` (`self.GetOwner`))
    (set `self.Hose` ConnectedHose)))

(fn `SetNoConnectedHose`
  (`self.SetConnectedHose` null))

(fn `SetOwningContainer`
  (params (OwningContainer :type "/Game/HoseSystem/Blueprints/Container_Component Object Reference"))
  (set `self.OwningContainer` OwningContainer))

(fn `StartPump`
  (bind (_hoseconnected _hose) (`self.GetConnectedHose`))
  (bind _owningcontainer (`self.OwningContainer`))
  (bind _inputconnection (`/Game/HoseSystem/Blueprints/HoseActor.GetInputConnection` _hose))
  (if (`Actor.HasAuthority` (`self.GetOwner`))
    (if (`self.GetIsConnectedAsInput`)
      (`/Engine/EditorBlueprintResources/StandardMacros.IsValid` _owningcontainer :!label _label
        (:`Is Valid`
          (if (or (`/Game/HoseSystem/Blueprints/Container_Component.InfiniteContents` _owningcontainer) (> (`/Game/HoseSystem/Blueprints/Container_Component.CurrentContents` _owningcontainer) 0.0))
            (set `self.IsPumping` true))))
      (elif _hoseconnected
        (`/Engine/EditorBlueprintResources/StandardMacros.IsValid` _inputconnection
          (:`Is Valid`
            (`self.StartPump` _inputconnection)))
        (else
          (goto _label))))))

(fn `StopPump`
  (bind (_hoseconnected _hose) (`self.GetConnectedHose`))
  (bind _inputconnection (`/Game/HoseSystem/Blueprints/HoseActor.GetInputConnection` _hose))
  (if (`Actor.HasAuthority` (`self.GetOwner`))
    (if (`self.GetIsConnectedAsInput`)
      (set `self.IsPumping` false)
      (elif _hoseconnected
        (`/Engine/EditorBlueprintResources/StandardMacros.IsValid` _inputconnection
          (:`Is Valid`
            (`self.StopPump` _inputconnection)))
        (else
          (set `self.IsPumping` false))))))

(fn `TogglePump`
  (if (`self.GetIsPumping`)
    (`self.StopPump`)
    (else
      (`self.StartPump`))))