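; Character component that spawns a water gun on the first-person mesh and paints wet-spot style marks where it shoots.
; On BeginPlay it attaches the gun and adds the weapon input mapping.
; Left input fires while held and right input toggles timed auto-fire, both driving the spray particles.
; Each shot traces from the camera, finds the hit UV and draws a circle into a render target, with RT_Test cleared on EndPlay.
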(event `self.ReceiveEndPlay`
  (params (EndPlayReason :type "EEndPlayReason Enum" :default "Destroyed"))
  (`KismetRenderingLibrary.ClearRenderTarget2D` "/Game/Game/Character/RenderTarget/RT_Test.RT_Test" (`TextureRenderTarget2D.ClearColor` (`self.Texture Render Target`))))

(event `self.ReceiveBeginPlay`
  (bind _bp_firstperson (`self.BP_FirstPerson`))
  (`|ExecutionSequence`
    (:`then_0`
      (bind _asbp_first_person_character (cast `/Game/Game/Character/Player/FirstPerson/Blueprints/BP_FirstPersonCharacter` (`self.GetOwner`)))
      (bind _output_get (set `self.BP_FirstPerson` _asbp_first_person_character))
      (bind _returnvalue (`|SpawnActorFromClass` (`self.WaterGunClass`) (`Actor.GetTransform` _output_get) "Undefined" "MultiplyWithRoot" null null))
      (bind _output_get_2 (set `self.BP_WaterGun` _returnvalue))
      (`Actor.K2_AttachToComponent` _output_get_2 (`/Game/Game/Character/Player/FirstPerson/Blueprints/BP_FirstPersonCharacter.FirstPersonMesh` _bp_firstperson) "GripPoint" "SnapToTarget" "SnapToTarget" "SnapToTarget" true)
      (set `/Game/Game/Character/Player/FirstPerson/Blueprints/BP_FirstPersonCharacter.bHasRifle` true _bp_firstperson))
    (:`then_1`
      (bind _bp_firstperson_2 (`self.BP_FirstPerson`)
        (:`then`
          (bind `_as玩家控制器` (cast `PlayerController` (`Pawn.GetController` _bp_firstperson_2)))
          (bind _returnvalue_2 (pcsubsystem `EnhancedInputLocalPlayerSubsystem` `_as玩家控制器`))
          (`/Engine/EditorBlueprintResources/StandardMacros.IsValid` _returnvalue_2
            (:`Is Valid`
              (`EnhancedInputSubsystemInterface.AddMappingContext` _returnvalue_2 "/Game/Game/Character/Player/FirstPerson/Input/IMC_Weapons.IMC_Weapons" 1 (struct)))))
        (:`else`)))))

(event `EnhancedInput|/Game/Game/Character/Player/FirstPerson/Input/Actions/IA_L_Shoot`
  (params (ActionValue :type Boolean) (ElapsedSeconds :type "Float (double-precision)") (TriggeredSeconds :type "Float (double-precision)") (InputAction :type "InputAction Object Reference" :default "/Game/Game/Character/Player/FirstPerson/Input/Actions/IA_L_Shoot.IA_L_Shoot"))
  (bind _ps_spray (`/Game/Game/WaterGun/BP_BaseWaterGun.PS_Spray` (`self.BP_WaterGun`)))
  (:`Triggered`
    (`self.ShootEvent`))
  (:`Started`
    (`self.SetActive` _ps_spray true false :!label _label))
  (:`Completed`
    (`self.SetActive` _ps_spray false false)))

(event `EnhancedInput|/Game/Game/Character/Player/FirstPerson/Input/Actions/IA_R_Shoot`
  (params (ActionValue :type Boolean) (ElapsedSeconds :type "Float (double-precision)") (TriggeredSeconds :type "Float (double-precision)") (InputAction :type "InputAction Object Reference" :default "/Game/Game/Character/Player/FirstPerson/Input/Actions/IA_R_Shoot.IA_R_Shoot"))
  (:`Started`
    (`/Engine/EditorBlueprintResources/StandardMacros.FlipFlop`
      (:`A`
        (bind _returnvalue (`KismetSystemLibrary.K2_SetTimerDelegate` (delegate `ShootEvent`) 0.1 true))
        (set `self.ShootTimerHandle` _returnvalue)
        (goto _label))
      (:`B`
        (`KismetSystemLibrary.K2_ClearAndInvalidateTimerHandle` (`self.ShootTimerHandle`))
        (`self.SetActive` (`/Game/Game/WaterGun/BP_BaseWaterGun.PS_Spray` (`self.BP_WaterGun`)) false false)))))

(event `ShootEvent`
  (bind _transformcomponent (`PlayerCameraManager.TransformComponent` (`GameplayStatics.GetPlayerCameraManager` 0)))
  (bind _returnvalue (`SceneComponent.K2_GetComponentLocation` _transformcomponent))
  (bind (_outhit _returnvalue_2) (`KismetSystemLibrary.LineTraceSingleForObjects` _returnvalue (+ _returnvalue (* (`SceneComponent.GetForwardVector` _transformcomponent) 2000.0)) (`|MakeArray` "ObjectTypeQuery1" :!type "EObjectTypeQuery Enum") true))
  (bind (_uv _returnvalue_3) (`GameplayStatics.FindCollisionUV` _outhit))
  (if (and _returnvalue_3 _returnvalue_2)
    (bind (_canvas _size) (`KismetRenderingLibrary.BeginDrawCanvasToRenderTarget` (`self.Texture Render Target`)))
    (`Canvas.K2_DrawPolygon` _canvas null (* _size _uv) (10.0 10.0) 50 (struct :`R` 1.0 :`G` 1.0 :`B` 1.0 :`A` 1.0))))