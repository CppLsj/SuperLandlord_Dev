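; BP_BaseWaterGun is a base water gun Blueprint with a skeletal mesh and a spray particle component.
; On BeginPlay it activates the spray and sets its world rotation once, with no later updates.
; The rotation is a look-at from the deprojected screen-center direction, scaled and used as a world position without the camera location added, toward the mesh's Muzzle socket.
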(event `self.ReceiveBeginPlay`
  (bind (_returnvalue_x _returnvalue_y) (`KismetMathLibrary.BreakVector2D` (* (`WidgetLayoutLibrary.GetViewportSize`) 0.5)))
  (`ActorComponent.SetActive` (`self.PS_Spray`) true false)
  (`SceneComponent.K2_SetWorldRotation` (`self.PS_Spray`) (`KismetMathLibrary.FindLookAtRotation` (* (`.WorldDirection` (`PlayerController.DeprojectScreenPositionToWorld` (`GameplayStatics.GetPlayerController` 0) _returnvalue_x _returnvalue_y)) 600.0) (`SceneComponent.GetSocketLocation` (`self.SkeletalMesh`) "Muzzle")) false false))

(fn `UserConstructionScript`)